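; Interactable Simon Says button puzzle, still a work in progress with empty click handlers for its nine buttons.
; Interact blends the view to the puzzle, freezes look and movement, and enables cursor clicks, while E restores normal player control.
; On interact, Button4 flashes green for two seconds before reverting to copper.
; Sequence and input checking are unfinished: other highlight nodes are disconnected and GetPressed always returns false.
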(event `Key|E`
  (params (Key :type "Key Structure"))
  (bind _returnvalue (`GameplayStatics.GetPlayerController` 0))
  (:`Pressed`
    (`PlayerController.SetViewTargetWithBlend` _returnvalue (`GameplayStatics.GetPlayerCharacter` 0) 0.3 "VTBlend_Linear" 0.0 false)
    (`Controller.ResetIgnoreLookInput` _returnvalue)
    (set `PlayerController.bEnableClickEvents` false _returnvalue)
    (set `PlayerController.bShowMouseCursor` false _returnvalue)
    (`CharacterMovementComponent.SetMovementMode` (`Character.CharacterMovement` (`GameplayStatics.GetPlayerCharacter` 0)) "MOVE_Walking" 0)
    (`WidgetBlueprintLibrary.SetInputMode_GameOnly` _returnvalue)
    (`self.DisableInput` _returnvalue)))

(event `/Player_Line_Trace/BI_Interaction.Interact`
  (bind _returnvalue (`GameplayStatics.GetPlayerController` 0))
  (bind _returnvalue_2 (`GameplayStatics.GetPlayerController` 0))
  (`|ExecutionSequence`
    (:`then_0`
      (`PlayerController.SetViewTargetWithBlend` _returnvalue_2 self 0.3 "VTBlend_Linear" 0.0 false)
      (`Controller.SetIgnoreLookInput` _returnvalue_2 true)
      (set `PlayerController.bEnableClickEvents` true _returnvalue_2)
      (set `PlayerController.bShowMouseCursor` true _returnvalue_2)
      (`CharacterMovementComponent.DisableMovement` (`Character.CharacterMovement` (`GameplayStatics.GetPlayerCharacter` 0)))
      (`self.EnableInput` _returnvalue)
      (`WidgetBlueprintLibrary.SetInputMode_GameAndUIEx` _returnvalue null))
    (:`then_1`
      (`PrimitiveComponent.SetMaterial` (`self.button4`) 0 "/Game/Unit_7_Content/Keypad/MI_KGreen.MI_KGreen" :!label _label)
      (`KismetSystemLibrary.Delay` 2.0)
      (`PrimitiveComponent.SetMaterial` (`self.button4`) 0 "/Game/StarterContent/Materials/M_Metal_Copper.M_Metal_Copper")
      (if (not true)
        (goto _label)))))

(event `self.button1.OnClicked`
  (params (TouchedComponent :type "PrimitiveComponent Object Reference") (ButtonPressed :type "Key Structure")))

(event `self.button2.OnClicked`
  (params (TouchedComponent :type "PrimitiveComponent Object Reference") (ButtonPressed :type "Key Structure")))

(event `self.button3.OnClicked`
  (params (TouchedComponent :type "PrimitiveComponent Object Reference") (ButtonPressed :type "Key Structure")))

(event `self.button4.OnClicked`
  (params (TouchedComponent :type "PrimitiveComponent Object Reference") (ButtonPressed :type "Key Structure")))

(event `self.button5.OnClicked`
  (params (TouchedComponent :type "PrimitiveComponent Object Reference") (ButtonPressed :type "Key Structure")))

(event `self.button6.OnClicked`
  (params (TouchedComponent :type "PrimitiveComponent Object Reference") (ButtonPressed :type "Key Structure")))

(event `self.button7.OnClicked`
  (params (TouchedComponent :type "PrimitiveComponent Object Reference") (ButtonPressed :type "Key Structure")))

(event `self.button8.OnClicked`
  (params (TouchedComponent :type "PrimitiveComponent Object Reference") (ButtonPressed :type "Key Structure")))

(event `self.button9.OnClicked`
  (params (TouchedComponent :type "PrimitiveComponent Object Reference") (ButtonPressed :type "Key Structure")))

(fn `Get Pressed`
  (returns (Correct :type Boolean))
  (return false))

(fn `UserConstructionScript`)